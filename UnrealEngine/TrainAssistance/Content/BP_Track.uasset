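; Train track actor that periodically sends a train along the track, with a text countdown and a warning indicator.
; Tick derives remaining seconds from a random delay, updating the text and a three-level situation that drives "occupied" and "urgent" parameters on the cube's dynamic material.
; At expiry, a DoOnce-guarded timeline offsets the train per update, then hides and repositions it and rolls a new hardcoded-range delay without resetting the start time.
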(event `self.ReceiveBeginPlay`
  (set `self.secondsTocome` (`KismetMathLibrary.RandomIntegerInRange` (`self.Min`) (`self.Max`)))
  (set `self.time` (`KismetMathLibrary.Now`))
  (`SceneComponent.SetVisibility` (`self.Train`) false false))

(event `self.ReceiveTick`
  (params (DeltaSeconds :type "Float (single-precision)"))
  (bind _returnvalue (- (`self.secondsTocome`) (`KismetMathLibrary.FTrunc` (`KismetMathLibrary.GetTotalSeconds` (- (`KismetMathLibrary.Now`) (`self.time`))))))
  (`self.setSituation` _returnvalue)
  (if (< _returnvalue 0)
    (`/Engine/EditorBlueprintResources/StandardMacros.DoOnce` false :!label _label
      (:`Completed`
        (`self.MoveTrain`)))))

(event `MoveTrain`
  (`SceneComponent.SetVisibility` (`self.Train`) true false)
  (`Timeline|Timeline_0` :!via `PlayFromStart`
    (:`Update`
      (`SceneComponent.K2_AddWorldOffset` (`self.Train`) (0.0 -100.0 0.0) false false))
    (:`Finished`
      (`self.StopTrain`)
      (goto _label :!via `Reset`))))

(event `StopTrain`
  (`SceneComponent.K2_AddWorldOffset` (`self.Train`) (0.0 0.0 0.0) false false)
  (set `self.secondsTocome` (`KismetMathLibrary.RandomIntegerInRange` 10 500))
  (`SceneComponent.SetVisibility` (`self.Train`) false false)
  (`SceneComponent.K2_SetWorldLocation` (`self.Train`) (`self.initialPosition`) false false))

(fn `getSecondsToComeATrain`)

(fn `setMaterialSituation`
  (params (dynamicSituationMaterial :type "MaterialInstanceDynamic Object Reference"))
  (`MaterialInstanceDynamic.SetScalarParameterValue` dynamicSituationMaterial "occupied" (`KismetMathLibrary.Conv_IntToDouble` (`KismetMathLibrary.SelectInt` 1 0 (`|EnumEquality` (`self.TrackSituation`) "NewEnumerator0"))))
  (`MaterialInstanceDynamic.SetScalarParameterValue` dynamicSituationMaterial "urgent" (`KismetMathLibrary.Conv_IntToDouble` (`KismetMathLibrary.SelectInt` 1 0 (`|EnumEquality` (`self.TrackSituation`) "NewEnumerator2"))))
  (set `self.dynamicSituationMaterial` dynamicSituationMaterial))

(fn `setSituation`
  (params (secondsToCome :type Integer))
  (bind _returnvalue (/ secondsToCome 60))
  (`TextRenderComponent.K2_SetText` (`self.TextRender`) (select `bool` (< secondsToCome 0) :`false` (`KismetTextLibrary.Conv_StringToText` (`KismetStringLibrary.Concat_StrStr` (`KismetStringLibrary.Conv_IntToString` _returnvalue) "  Minuntes  " (`KismetStringLibrary.Conv_IntToString` (- secondsToCome (* _returnvalue 60))) "  Seconds   " "For  " "Train")) :`true` "WARNING! TRAIN COMING"))
  (set `self.TrackSituation` (select `bool` (< secondsToCome 120) :`false` (select `bool` (< secondsToCome 300) :`false` "NewEnumerator1" :`true` "NewEnumerator0" :!type "/Game/E_TrackSituation Enum") :`true` "NewEnumerator2"))
  (`self.setMaterialSituation` (`self.dynamicSituationMaterial`)))

(fn `UserConstructionScript`
  (bind _cube (`self.Cube`))
  (bind _returnvalue (`PrimitiveComponent.CreateDynamicMaterialInstance` _cube 0 (`PrimitiveComponent.GetMaterial` _cube 0) "None"))
  (`self.setMaterialSituation` _returnvalue))