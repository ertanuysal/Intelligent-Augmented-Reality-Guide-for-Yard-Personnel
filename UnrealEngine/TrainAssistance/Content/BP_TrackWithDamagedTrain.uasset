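; Track actor, named for a damaged train, that shows its track situation and triggers an assistance prompt for the VR worker.
; The construction script creates a dynamic material on the Cube and sets its "occupied" and "urgent" scalar parameters from the TrackSituation enum.
; The first time a VRPawnWorker overlaps the Box, it plays the OpenAsistance animation on that pawn's W_Main HUD widget.
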(event `self.Box.OnComponentBeginOverlap`
  (params (OverlappedComponent :type "PrimitiveComponent Object Reference") (OtherActor :type "Actor Object Reference") (OtherComp :type "PrimitiveComponent Object Reference") (OtherBodyIndex :type Integer) (bFromSweep :type Boolean) (SweepResult :type "HitResult Structure (by ref)"))
  (bind _asvrpawn_worker (cast `/Game/VRPawnWorker` OtherActor))
  (`/Engine/EditorBlueprintResources/StandardMacros.DoOnce` false
    (:`Completed`
      (bind _returnvalue (`WidgetComponent.GetWidget` (`/Game/VRPawnWorker.HUD` _asvrpawn_worker)))
      (bind _asw_main (cast `/Game/Widget/W_Main` _returnvalue))
      (`UserWidget.PlayAnimation` _returnvalue (`/Game/Widget/W_Main.openAsistance` _asw_main) 0.0 1 "Forward" 1.0 false))))

(fn `setMaterialSituation`
  (params (dynamicSituationMaterial :type "MaterialInstanceDynamic Object Reference"))
  (`MaterialInstanceDynamic.SetScalarParameterValue` dynamicSituationMaterial "occupied" (`KismetMathLibrary.Conv_IntToDouble` (`KismetMathLibrary.SelectInt` 1 0 (`|EnumEquality` (`self.TrackSituation`) "NewEnumerator0"))))
  (`MaterialInstanceDynamic.SetScalarParameterValue` dynamicSituationMaterial "urgent" (`KismetMathLibrary.Conv_IntToDouble` (`KismetMathLibrary.SelectInt` 1 0 (`|EnumEquality` (`self.TrackSituation`) "NewEnumerator2"))))
  (set `self.dynamicSituationMaterial` dynamicSituationMaterial))

(fn `UserConstructionScript`
  (bind _cube (`self.Cube`))
  (bind _returnvalue (`PrimitiveComponent.CreateDynamicMaterialInstance` _cube 0 (`PrimitiveComponent.GetMaterial` _cube 0) "None"))
  (`self.setMaterialSituation` _returnvalue))